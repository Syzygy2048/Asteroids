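; Player controller for an Asteroids game that turns input actions into commands on the player pawn.
; Press and release events for left, right, forward, back and shoot set boolean held flags.
; Tick checks each flag every frame and calls the matching pawn input function, so held inputs, including fire, repeat continuously.
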(event EventBeginPlay)

(event EventTick
  (params (DeltaSeconds :type Float%20%28single-precision%29))
  (bind _player_pawn (Variables|Default|GetPlayer%20Pawn))
  (if (Variables|Default|Getleft%20pressed)
    (Default|OnInputLeft _player_pawn))
  (if (Variables|Default|Getright%20pressed)
    (Default|OnInputRight _player_pawn))
  (if (Variables|Default|Getforward%20pressed)
    (Default|OnInputForward _player_pawn))
  (if (Variables|Default|Getback%20pressed)
    (Default|OnInputBack _player_pawn))
  (if (Variables|Default|Getfire%20pressed)
    (Default|OnInputFire _player_pawn)))

(event Input|ActionEvents|InputActionLeft
  (params (Key :type Key%20Structure :default "AnyKey"))
  (:Pressed
    (Variables|Default|Setleft%20pressed true))
  (:Released
    (Variables|Default|Setleft%20pressed false)))

(event Input|ActionEvents|InputActionRight
  (params (Key :type Key%20Structure :default "AnyKey"))
  (:Pressed
    (Variables|Default|Setright%20pressed true))
  (:Released
    (Variables|Default|Setright%20pressed false)))

(event Input|ActionEvents|InputActionForward
  (params (Key :type Key%20Structure :default "AnyKey"))
  (:Pressed
    (Variables|Default|Setforward%20pressed true))
  (:Released
    (Variables|Default|Setforward%20pressed false)))

(event Input|ActionEvents|InputActionBack
  (params (Key :type Key%20Structure :default "AnyKey"))
  (:Pressed
    (Variables|Default|Setback%20pressed true))
  (:Released
    (Variables|Default|Setback%20pressed false)))

(event Input|ActionEvents|InputActionShoot
  (params (Key :type Key%20Structure :default "AnyKey"))
  (:Pressed
    (Variables|Default|Setfire%20pressed true))
  (:Released
    (Variables|Default|Setfire%20pressed false)))

(fn ConstructionScript)