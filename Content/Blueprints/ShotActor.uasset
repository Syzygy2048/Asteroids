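; Projectile actor that fires itself forward and sticks to debris it hits.
; BeginPlay applies a large physics impulse to the bullet sprite along its facing.
; On hit it ignores other shots; against a Debris1Actor it attaches in place, applies damage and sets IsAttached.
; Logic for sticking to already-attached shots is disconnected, and the TriggerVolume end-overlap check does nothing after its cast.
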(event OnComponentEndOverlap(Bullet_Sprite)
  (params (OtherActor :type Actor%20Object%20Reference) (OtherComp :type Primitive%20Component%20Object%20Reference) (OtherBodyIndex :type Integer))
  (Utilities|Casting|CastToTriggerVolume OtherActor))

(event OnComponentHit(Bullet_Sprite)
  (params (OtherActor :type Actor%20Object%20Reference) (OtherComp :type Primitive%20Component%20Object%20Reference) (NormalImpulse :type Vector :default "0, 0, 0") (Hit :type Hit%20Result%20Structure%20%28by%20ref%29))
  (bind _asshot_actor (Utilities|Casting|CastToShotActor OtherActor)
    (:CastFailed
      (bind _asdebris_1actor (Utilities|Casting|CastToDebris1Actor OtherActor))
      (Class|Actor|AttachRootComponenttoActor self _asdebris_1actor "None" "KeepWorldPosition" true)
      (Game|Damage|ApplyDamage _asdebris_1actor 1e+01 0 0)
      (Variables|Default|SetisAttached true))))

(event EventBeginPlay
  (bind _bullet_sprite (Variables|Default|GetBullet_Sprite))
  (Physics|AddImpulse _bullet_sprite (* (Math|Rotator|GetRotationXVector (Transformation|GetWorldRotation _bullet_sprite)) 1.5e+05) "None" false))

(event EventActorBeginOverlap
  (params (OtherActor :type Actor%20Object%20Reference)))

(event EventTick
  (params (DeltaSeconds :type Float%20%28single-precision%29)))

(fn ConstructionScript)