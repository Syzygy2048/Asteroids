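; Player spaceship pawn for an Asteroids game, possessed on BeginPlay by player controller 0, which receives a reference to it.
; OnInput functions rotate the ship in fixed yaw steps and push the sprite along its up vector with a physics impulse; back is empty.
; Fire spawns a shot ahead of the nose, rate-limited by a next-shot timestamp.
; Debug prints remain in forward thrust and the Forward input event.
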(event EventBeginPlay
  (bind _returnvalue (Game|GetPlayerController 0))
  (bind _self self)
  (Pawn|Possess _returnvalue _self)
  (bind _asasteroids_player_controller (Utilities|Casting|CastToAsteroidsPlayerController _returnvalue))
  (Variables|/Game/Blueprints/AsteroidsPlayerController.AsteroidsPlayerController_C|SetPlayer%20Pawn _asasteroids_player_controller _self))

(event EventActorBeginOverlap
  (params (OtherActor :type Actor%20Object%20Reference)))

(event EventTick
  (params (DeltaSeconds :type Float%20%28single-precision%29)))

(event Input|ActionEvents|InputActionForward
  (params (Key :type Key%20Structure :default "AnyKey"))
  (:Pressed
    (Development|PrintString "Hello")))

(fn ConstructionScript)

(fn OnInputLeft
  (Class|Actor|AddActorWorldRotation "-4.000000, 0, 0"))

(fn OnInputRight
  (Class|Actor|AddActorWorldRotation "4.000000,0.000000, 0"))

(fn OnInputForward
  (bind _spaceship_sprite (Variables|Default|GetSpaceship_Sprite))
  (bind _returnvalue (Math|Vector|GetUpVector _spaceship_sprite))
  (bind _returnvalue_2 (* _returnvalue 5e+03))
  (bind (_x _y _z) (Math|Vector|BreakVector _returnvalue_2))
  (Development|PrintString (Utilities|String|Append (Utilities|String|ToString(Float) _x) ", " (Utilities|String|ToString(Float) _y) ", " (Utilities|String|ToString(Float) _z)))
  (Physics|AddImpulse _spaceship_sprite _returnvalue_2 "None" false))

(fn OnInputBack)

(fn OnInputFire
  (bind _self self)
  (bind _spaceship_sprite (Variables|Default|GetSpaceship_Sprite))
  (bind _returnvalue (Math|Vector|GetUpVector _spaceship_sprite))
  (if (< (Variables|Default|GettimeOfNextShot) (Math|DateTime|Now))
    (Game|SpawnActorfromClass "/Game/Blueprints/ShotActor.ShotActor_C" (Math|Transform|MakeTransform (+ (Transformation|GetWorldLocation _spaceship_sprite) (* _returnvalue 4e+02)) (Math|Conversions|RotationFromXVector _returnvalue)) "AlwaysSpawn" _self _self)
    (Variables|Default|SettimeOfNextShot (+ (Math|DateTime|Now) (Variables|Default|GetfireRateTimespan)))))