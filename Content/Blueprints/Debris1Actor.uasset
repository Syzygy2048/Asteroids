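; Debris actor with a sprite and a health value that reacts when damage runs it out.
; AnyDamage subtracts from Health, then tests the updated value minus Damage again, so the break triggers once that falls below zero.
; The break applies a radial impulse to its own sprite at the actor location, with debug print and circle.
; DestroyActor is unwired, so the actor persists; hit handlers are empty.
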(event OnComponentHit(Derbis1_Sprite)
  (params (OtherActor :type Actor%20Object%20Reference) (OtherComp :type Primitive%20Component%20Object%20Reference) (NormalImpulse :type Vector) (Hit :type Hit%20Result%20Structure%20%28by%20ref%29)))

(event EventBeginPlay)

(event EventActorBeginOverlap
  (params (OtherActor :type Actor%20Object%20Reference)))

(event EventTick
  (params (DeltaSeconds :type Float%20%28single-precision%29)))

(event Game|Damage|EventAnyDamage
  (params (Damage :type Float%20%28single-precision%29) (DamageType :type Damage%20Type%20Object%20Reference) (InstigatedBy :type Controller%20Object%20Reference) (DamageCauser :type Actor%20Object%20Reference))
  (bind _returnvalue (Transformation|GetActorLocation))
  (bind _newvar_0 (Variables|Default|GetNewVar_0))
  (Variables|Default|Sethealth (- (Variables|Default|Gethealth) Damage))
  (if (< (- (Variables|Default|Gethealth) Damage) 0.0)
    (Physics|AddRadialImpulse (Variables|Default|GetDerbis1_Sprite) _returnvalue _newvar_0 _newvar_0 "RIF_Constant" false)
    (Development|PrintString (Utilities|String|ToString(Vector) _returnvalue))
    (Rendering|Debug|DrawDebugCircle _returnvalue _newvar_0 12 "(R=1.000000,G=0.000000,B=0.076571,A=1.000000)" 1.0 0.0 "1.000000,1.000000,0.000000" "0.000000,0.000000,1.000000")))

(fn ConstructionScript)

(fn OnGettingHit)